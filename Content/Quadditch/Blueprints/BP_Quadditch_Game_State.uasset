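; Game state for Quadditch, a team drone game, tracking quadcopters, play state and match time.
; NsMsg registers drones by namespace, refreshing a known drone's check-in time or spawning a new BP_Quadcopter_A on alternating teams and updating the admin list.
; The Playing RepNotify runs a timer-driven countdown widget, which then sets drone controllability, starts the game clock and has the game mode assign the ball.
; Clock expiry only prints game over.
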(event EventTick
  (params (DeltaSeconds :type Float%20%28single-precision%29)))

(event EventBeginPlay
  (bind _returnvalue (Game|ConstructObjectfromClass "/Game/Quadditch/UI/countdown.countdown_C" self))
  (Variables|Default|Setcountdown%20widget _returnvalue))

(fn ConstructionScript)

(fn NsMsg
  (params (string%20msg :type String))
  (bind _namespaces (Variables|Default|GetNamespaces))
  ;[1 1 1] check if the drone is already in the game
  (if (Utilities|Array|ContainsItem _namespaces string%20msg)
    ;[1 1 1] update the drone's last check-in time
    (bind _array_element (Utilities|Array|ForEachLoopwithBreak (Variables|Default|GetDrones) :!label _label)
      (:LoopBody
        (if (Utilities|Enum|Equal(Enum) (Variables|/Game/Quadcopters/Blueprints/BP_Quadcopter_A.BP_Quadcopter_A_C|GetNamespace _array_element) string%20msg)
          (Variables|/Game/Quadcopters/Blueprints/BP_Quadcopter_A.BP_Quadcopter_A_C|Setlast%20alive _array_element (Math|DateTime|Now))
          (goto _label Break))))
    (else
      ;[1 1 1] spawn a drone having the new namespace
      (Utilities|Array|Add _namespaces string%20msg)
      (bind _returnvalue (Game|SpawnActorfromClass "/Game/Quadcopters/Blueprints/BP_Quadcopter_A.BP_Quadcopter_A_C" (Math|Transform|MakeTransform "0, 0,700.000000") "AdjustIfPossibleButAlwaysSpawn" self 0))
      (Default|Init _returnvalue string%20msg)
      (CallFunction|IncrementTeam)
      (bind _output_get (Variables|/Game/Quadcopters/Blueprints/BP_Quadcopter_A.BP_Quadcopter_A_C|Setteam _returnvalue (Variables|Default|Getteam%20toggle)))
      ;;[1 1 1] (obsolete) set quaffle respawn area
      (Variables|/Game/Quadcopters/Blueprints/BP_Quadcopter_A.BP_Quadcopter_A_C|Setquaffle%20spawn _returnvalue (Utilities|Select :Index _output_get :NewEnumerator0 (Variables|Default|Getquaffle_spawn%20red) :NewEnumerator1 (Variables|Default|Getquaffle_spawn%20blue)))
      (Utilities|Array|Add (Variables|Default|GetDrones) _returnvalue)
      (CallFunction|RefreshAdminUi))))

(fn RefreshAdminUi
  (bind _asbp_ros_game (Utilities|Casting|CastToBP_ROS_GAME (Game|GetGameInstance)))
  (if (Variables|/Game/ROS/Blueprints/BP_ROS_GAME.BP_ROS_GAME_C|Getis%20admin _asbp_ros_game)
    (bind _asbp_spectator (Utilities|Casting|CastToBP_Spectator (Pawn|GetControlledPawn (Game|GetPlayerController 0))))
    (Default|RefreshDroneList (Variables|/Game/Quadditch/Blueprints/BP_Spectator.BP_Spectator_C|Getadmin%20control%20ui _asbp_spectator))))

(fn OnRepPlaying
  (bind _returnvalue (Utilities|Time|SetTimerbyFunctionName 0 "game countdown" 1.0 true))
  (Variables|Default|Setcountdown%20timer _returnvalue))

(fn GameCountdown
  (bind _countdown_widget (Variables|Default|Getcountdown%20widget))
  (bind _count (Variables|Default|Getcount))
  (UserInterface|Viewport|AddtoViewport _countdown_widget 0)
  (Widget|SetVisibility _countdown_widget "Visible")
  (if (> _count 0)
    (Variables|/Game/Quadditch/UI/countdown.countdown_C|Setcount%20text%20val _countdown_widget (Utilities|String|ToString(Integer) _count))
    (Math|Integer|DecrementInt (Variables|Default|Getcount) :!label _label)
    (else
      (if (Variables|Default|Getplaying)
        (Variables|/Game/Quadditch/UI/countdown.countdown_C|Setcount%20text%20val _countdown_widget "Start!")
        (else
          (Variables|/Game/Quadditch/UI/countdown.countdown_C|Setcount%20text%20val _countdown_widget "Finish!")))
      (if (< (Variables|Default|Getcount) 0)
        (Utilities|Time|ClearandInvalidateTimerbyHandle (Variables|Default|Getcountdown%20timer))
        (for _array_element (Variables|Default|GetDrones)
          (Variables|/Game/Quadcopters/Blueprints/BP_Quadcopter_A.BP_Quadcopter_A_C|Setcontrollable _array_element (Variables|Default|Getplaying)))
        (Widget|RemovefromParent (Variables|Default|Getcountdown%20widget))
        (Variables|Default|Setgame%20time%20min 5)
        (Variables|Default|Setgame%20time%20sec 0)
        (bind _returnvalue (Utilities|Time|SetTimerbyFunctionName 0 "game clock tick" 1.0 true))
        (Variables|Default|Setcountdown%20timer _returnvalue)
        (bind _asbp_quadditch_game_mode (Utilities|Casting|CastToBP_Quadditch_Game_Mode (Game|GetGameMode)))
        (Default|AssignBall _asbp_quadditch_game_mode "NewEnumerator0")
        (else
          (goto _label))))))

(fn IncrementTeam
  (Variables|Default|Setteam%20toggle (select (>= (Math|Conversions|ToInteger(Byte) (+ (Variables|Default|Getteam%20toggle) 1)) (|GetNumEnumEntries)) (Utilities|Enum|ByteToEnumTeamEnum) (Utilities|Enum|ByteToEnumTeamEnum (+ (Variables|Default|Getteam%20toggle) 1)))))

(fn GameClockTick
  (bind _result (Math|Integer|DecrementInt (Variables|Default|Getgame%20time%20sec))
    (:%20%20
      (if (< _result 0)
        (if (> (Variables|Default|Getgame%20time%20min) 0)
          (Variables|Default|Setgame%20time%20sec 59)
          (Math|Integer|DecrementInt (Variables|Default|Getgame%20time%20min))
          (else
            (Development|PrintString "GAME OVER")))))))