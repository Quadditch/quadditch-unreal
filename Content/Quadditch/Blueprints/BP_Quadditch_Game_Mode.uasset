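; Game mode for Quadditch, a ROS-linked team drone game, handling player join and exit, ball assignment and scoring.
; On login it connects to ROS and possesses a new spectator pawn; on logout the player state ejects the drone.
; BeginPlay subscribes to the ROS /alive topic and forwards messages to the game state.
; AssignBall gives the ball once to a random drone on a team; IncrementScore updates red or blue scores.
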(event Custom|string%20ns%20msg
  (params (val :type String))
  (bind _asbp_quadditch_game_state (Utilities|Casting|CastToBP_Quadditch_Game_State (Game|GetGameState)))
  (Default|NsMsg _asbp_quadditch_game_state val))

(event EventBeginPlay
  (Development|PrintString "BeginPlay triggered!" true true "(R=0.000000,G=0.660000,B=1.000000,A=1.000000)" 5.0)
  (bind _asbp_ros_game (Utilities|Casting|CastToBP_ROS_GAME (Game|GetGameInstance)))
  (if (Variables|/Script/ROSIntegration.ROSIntegrationGameInstance|GetbConnectToROS _asbp_ros_game)
    (bind _returnvalue (Game|ConstructObjectfromClass "/Game/ROS/Blueprints/BP_ROS_String_Sub.BP_ROS_String_Sub_C" self))
    (Development|PrintString "Subscribing to /alive")
    (Default|InitSub _returnvalue "/alive")
    (EventDispatchers|BindEventtoUpdateDispatcher _returnvalue (delegate Custom|string%20ns%20msg))))

(event EventPostLogin
  (params (NewPlayer :type Player%20Controller%20Object%20Reference))
  (Development|PrintString "OnPostLogin!" true true "(R=0.000000,G=0.660000,B=1.000000,A=1.000000)" 5.0)
  (bind _asbp_ros_game (Utilities|Casting|CastToBP_ROS_GAME (Game|GetGameInstance)))
  (Development|PrintString "Connecting to ROS" true true "(R=0.000000,G=0.660000,B=1.000000,A=1.000000)" 3.0)
  (if (Variables|/Script/ROSIntegration.ROSIntegrationGameInstance|GetbConnectToROS _asbp_ros_game)
    (Development|PrintString "Successfully connected to ROS." true true "(R=0.000000,G=0.660000,B=1.000000,A=1.000000)" 5.0)
    ;[1 1 1] spawn spectator by default. This class will continuously try to take control of an available drone
    (bind _returnvalue (Game|SpawnActorfromClass "/Game/Quadditch/Blueprints/BP_Spectator.BP_Spectator_C" (Math|Transform|MakeTransform "0, 0,100.000000") "Undefined" NewPlayer 0))
    (Pawn|Possess NewPlayer _returnvalue)
    (else
      (Development|PrintString "Failed to connect to ROS." true true "(R=0.000000,G=0.660000,B=1.000000,A=1.000000)" 1.2e+02))))

(event EventOnLogout
  (params (ExitingController :type Controller%20Object%20Reference))
  (Development|PrintString "Trying a graceful exit")
  (bind _asbp_quadditch_player_state (Utilities|Casting|CastToBP_Quadditch_Player_State (Variables|/Script/Engine.Controller|GetPlayerState ExitingController)))
  (Development|PrintString (Utilities|GetDisplayName (Variables|/Script/Engine.PlayerState|GetPawnPrivate _asbp_quadditch_player_state)))
  (bind _asbp_quadcopter_a (Utilities|Casting|CastToBP_Quadcopter_A))
  (Default|EjectDrone _asbp_quadditch_player_state _asbp_quadcopter_a ExitingController))

(fn ConstructionScript)

(fn AssignBall
  (params (team :type TeamEnum%20Enum :default "NewEnumerator0"))
  (bind _drones_on_team (LocalVariables|Getdrones%20on%20team))
  ;[1 1 1] make sure we don't accidentally assign the ball twice
  (if (not (Variables|Default|Getball%20assigned))
    (Variables|Default|Setball%20assigned true)
    ;[1 1 1] find all drones on desired team
    (bind _asbp_quadditch_game_state (Utilities|Casting|CastToBP_Quadditch_Game_State (Game|GetGameState)))
    (Utilities|Array|Clear (LocalVariables|Getdrones%20on%20team))
    (for _array_element (Variables|/Game/Quadditch/Blueprints/BP_Quadditch_Game_State.BP_Quadditch_Game_State_C|GetDrones _asbp_quadditch_game_state)
      (if (Utilities|Enum|Equal(Enum) (Variables|/Game/Quadcopters/Blueprints/BP_Quadcopter_A.BP_Quadcopter_A_C|Getteam _array_element) team)
        (Utilities|Array|Add (LocalVariables|Getdrones%20on%20team) _array_element)))
    ;[1 1 1] randomly assign ball to one drone on that team
    (Variables|/Game/Quadcopters/Blueprints/BP_Quadcopter_A.BP_Quadcopter_A_C|Sethas_ball (Utilities|Array|Get(acopy) _drones_on_team (Math|Random|RandomIntegerinRange 0 (- (Utilities|Array|Length _drones_on_team) 1))) true)))

(fn IncrementScore
  (params (team :type TeamEnum%20Enum :default "NewEnumerator0"))
  (bind _asbp_quadditch_game_state (Utilities|Casting|CastToBP_Quadditch_Game_State (Game|GetGameState)))
  (Math|Integer|IncrementInt (Utilities|Select :Index team :NewEnumerator0 (Variables|/Game/Quadditch/Blueprints/BP_Quadditch_Game_State.BP_Quadditch_Game_State_C|Getscore_red _asbp_quadditch_game_state) :NewEnumerator1 (Variables|/Game/Quadditch/Blueprints/BP_Quadditch_Game_State.BP_Quadditch_Game_State_C|Getscore_blue _asbp_quadditch_game_state))))