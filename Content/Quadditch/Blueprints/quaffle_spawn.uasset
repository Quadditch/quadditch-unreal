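; Quaffle spawn point that hands a quaffle to quadcopters flying into it in a Quidditch-style game.
; On capsule overlap, a BP_Quadcopter_A without a ball gets HasBall set and its HeldQuaffle shown, with no availability check.
; The pickup decrements QuafflesAvailable and shows QuaffleMesh only if the count is zero or less, which appears inverted.
; SpawnQuaffle increments the count and shows the mesh.
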(event OnComponentBeginOverlap(CollisionCapsule1)
  (params (OverlappedComponent :type Primitive%20Component%20Object%20Reference) (OtherActor :type Actor%20Object%20Reference) (OtherComp :type Primitive%20Component%20Object%20Reference) (OtherBodyIndex :type Integer) (bFromSweep :type Boolean) (SweepResult :type Hit%20Result%20Structure%20%28by%20ref%29))
  (bind _asbp_quadcopter_a (Utilities|Casting|CastToBP_Quadcopter_A OtherActor))
  (if (not (Variables|/Game/Quadcopters/Blueprints/BP_Quadcopter_A.BP_Quadcopter_A_C|Gethas_ball _asbp_quadcopter_a))
    (Variables|/Game/Quadcopters/Blueprints/BP_Quadcopter_A.BP_Quadcopter_A_C|Sethas_ball _asbp_quadcopter_a true)
    (Rendering|SetVisibility (Variables|/Game/Quadcopters/Blueprints/BP_Quadcopter_A.BP_Quadcopter_A_C|Getheld_quaffle _asbp_quadcopter_a) true false)
    (bind _result (Math|Integer|DecrementInt (Variables|Default|Getquaffles%20available))
      (:%20%20
        (Rendering|SetVisibility (Variables|Default|Getquaffle%20mesh) (<= _result 0) false)))))

(event EventBeginPlay)

(event EventTick
  (params (DeltaSeconds :type Float%20%28single-precision%29)))

(fn ConstructionScript)

(fn SpawnQuaffle
  (Math|Integer|IncrementInt (Variables|Default|Getquaffles%20available)
    (:%20%20
      (Rendering|SetVisibility (Variables|Default|Getquaffle%20mesh) true false))))