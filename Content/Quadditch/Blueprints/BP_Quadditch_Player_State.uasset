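; Player state for Quadditch that keeps a player in control of a quadcopter drone.
; Every tick, if the game instance flags a player and player 0's pawn is not a quadcopter, it possesses the first free drone in the game state's drone list.
; An eject event, noted as likely unused, moves a controller to a new spectator if its drone is possessed, then destroys that drone.
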(event Custom|eject%20drone
  (params (dead%20drone :type BP%20Quadcopter%20A%20Object%20Reference) (ejected%20controller :type Controller%20Object%20Reference))
  ;[1 1 1] probably useful for graceful disconnects but I don't think it's currently used
  (if (Variables|/Game/Quadcopters/Blueprints/BP_Quadcopter_A.BP_Quadcopter_A_C|Getis%20possessed dead%20drone)
    (bind _returnvalue (Game|SpawnActorfromClass "/Game/Quadditch/Blueprints/BP_Spectator.BP_Spectator_C" (Math|Transform|MakeTransform "0, 0, 0") "Undefined" 0 0))
    (Pawn|Possess ejected%20controller _returnvalue))
  (Actor|DestroyActor dead%20drone))

(event Custom|possess%20drone
  (params (pc :type Player%20Controller%20Object%20Reference))
  ;[1 1 1] Possess an unpossessed drone
  (bind _asbp_quadditch_game_state (Utilities|Casting|CastToBP_Quadditch_Game_State (Game|GetGameState)))
  (bind _array_element (Utilities|Array|ForEachLoopwithBreak (Variables|/Game/Quadditch/Blueprints/BP_Quadditch_Game_State.BP_Quadditch_Game_State_C|GetDrones _asbp_quadditch_game_state) :!label _label)
    (:LoopBody
      (if (not (Variables|/Game/Quadcopters/Blueprints/BP_Quadcopter_A.BP_Quadcopter_A_C|Getis%20possessed _array_element))
        (Pawn|Possess pc _array_element)
        (goto _label Break)))))

(event EventBeginPlay)

(event EventTick
  (params (DeltaSeconds :type Float%20%28single-precision%29))
  ;[1 1 1] If not drone, try to be drone
  (bind _asbp_ros_game (Utilities|Casting|CastToBP_ROS_GAME (Game|GetGameInstance)))
  (if (Variables|/Game/ROS/Blueprints/BP_ROS_GAME.BP_ROS_GAME_C|Getis%20player _asbp_ros_game)
    (Utilities|Casting|CastToBP_Quadcopter_A (Game|Player|GetPlayerPawn 0)
      (:CastFailed
        (CallFunction|PossessDrone (Game|GetPlayerController 0))))))

(fn ConstructionScript)