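; Bludger is a Quidditch-style ball actor that homes in on a target.
; Each tick, while TargetLocked is set, it overwrites the Ball's physics linear velocity to point at the Target's BodyMesh1 at a fixed Speed.
; The file shows no logic for acquiring or releasing the target, and its BeginPlay and overlap events are empty.
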(event EventBeginPlay)

(event Collision|EventActorBeginOverlap
  (params (OtherActor :type Actor%20Object%20Reference)))

(event EventTick
  (params (DeltaSeconds :type Float%20%28single-precision%29))
  (if (Variables|Default|Gettarget%20locked)
    (Physics|SetPhysicsLinearVelocity (Variables|Default|Getball) (* (Math|Vector|Normalize (- (Transformation|GetWorldLocation (Variables|/Game/Quadcopters/Blueprints/BP_Quadcopter_A.BP_Quadcopter_A_C|GetBodyMesh_1 (Variables|Default|Gettarget))) (Transformation|GetWorldLocation (Variables|Default|Getball)))) (Variables|Default|Getspeed)) false "None")))

(fn ConstructionScript)