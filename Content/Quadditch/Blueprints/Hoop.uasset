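; Team-owned Quadditch goal hoop, coloured red or blue, that detects overlapping Quaffles each tick and on actor overlap.
; A Quaffle adjusts its thrower's score by team, credits the opposing team through the game mode, then is destroyed.
; Each goal spawns confetti and hands the ball to the owning team's nearest drone.
; The emissive glow fade is unconnected, so the intensity set on scoring never reaches the material.
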(event Custom|hoop%20effects
  (Variables|Default|SetEmissive%20Intensity 1e+01)
  (Effects|SpawnEmitteratLocation "/Game/Quadditch/Materials/confetti_particles.confetti_particles" (Transformation|GetActorLocation) "0, 0, 0" "3.000000,3.000000,3.000000"))

(event Custom|restore%20ball
  (Variables|Default|Setclosest%20dist 1.8647120722022892e+18)
  (bind _asbp_quadditch_game_state (Utilities|Casting|CastToBP_Quadditch_Game_State (Game|GetGameState)))
  (for _array_element (Variables|/Game/Quadditch/Blueprints/BP_Quadditch_Game_State.BP_Quadditch_Game_State_C|GetDrones _asbp_quadditch_game_state)
    (if (Utilities|Enum|Equal(Enum) (Variables|/Game/Quadcopters/Blueprints/BP_Quadcopter_A.BP_Quadcopter_A_C|Getteam _array_element) (Variables|Default|Getowning_team))
      (if (< (Math|Vector|VectorLength (- (Transformation|GetActorLocation) (Transformation|GetActorLocation _array_element))) (Variables|Default|Getclosest%20dist))
        (Variables|Default|Setclosest _array_element)
        (Variables|Default|Setclosest%20dist (Math|Vector|VectorLength (- (Transformation|GetActorLocation) (Transformation|GetActorLocation _array_element)))))))
  (Variables|/Game/Quadcopters/Blueprints/BP_Quadcopter_A.BP_Quadcopter_A_C|Sethas_ball (Variables|Default|Getclosest) true))

(event EventBeginPlay)

(event Collision|EventActorBeginOverlap
  (params (OtherActor :type Actor%20Object%20Reference))
  (bind _owning_team (Variables|Default|Getowning_team))
  (for _array_element (Collision|GetOverlappingActors (Variables|Default|GetCylinder) "/Game/Quadditch/Blueprints/Quaffle.Quaffle_C" :!class /Script/Engine.PrimitiveComponent)
    (bind _asbp_quadcopter_a (Utilities|Casting|CastToBP_Quadcopter_A (Game|GetInstigator _array_element)))
    (if (!= _owning_team (Variables|/Game/Quadcopters/Blueprints/BP_Quadcopter_A.BP_Quadcopter_A_C|Getteam _asbp_quadcopter_a))
      (Math|Integer|IncrementInt (Variables|/Game/Quadcopters/Blueprints/BP_Quadcopter_A.BP_Quadcopter_A_C|Getscore _asbp_quadcopter_a)
        (:%20%20
          _))
      (else
        (Math|Integer|DecrementInt (Variables|/Game/Quadcopters/Blueprints/BP_Quadcopter_A.BP_Quadcopter_A_C|Getscore _asbp_quadcopter_a)
          (:%20%20
            _))))
    (bind _asbp_quadditch_game_mode (Utilities|Casting|CastToBP_Quadditch_Game_Mode (Game|GetGameMode)))
    (Default|IncrementScore _asbp_quadditch_game_mode (Utilities|Select :Index _owning_team :NewEnumerator0 "NewEnumerator1" :NewEnumerator1 "NewEnumerator0"))
    (Actor|DestroyActor _array_element)
    (CallFunction|HoopEffects)
    (CallFunction|RestoreBall)))

(event EventTick
  (params (DeltaSeconds :type Float%20%28single-precision%29))
  (bind _owning_team (Variables|Default|Getowning_team))
  (for _array_element (Collision|GetOverlappingActors (Variables|Default|GetCylinder) "/Game/Quadditch/Blueprints/Quaffle.Quaffle_C" :!class /Script/Engine.PrimitiveComponent)
    (bind _asbp_quadcopter_a (Utilities|Casting|CastToBP_Quadcopter_A (Game|GetInstigator _array_element)))
    (if (!= _owning_team (Variables|/Game/Quadcopters/Blueprints/BP_Quadcopter_A.BP_Quadcopter_A_C|Getteam _asbp_quadcopter_a))
      (Math|Integer|IncrementInt (Variables|/Game/Quadcopters/Blueprints/BP_Quadcopter_A.BP_Quadcopter_A_C|Getscore _asbp_quadcopter_a)
        (:%20%20
          _))
      (else
        (Math|Integer|DecrementInt (Variables|/Game/Quadcopters/Blueprints/BP_Quadcopter_A.BP_Quadcopter_A_C|Getscore _asbp_quadcopter_a)
          (:%20%20
            _))))
    (bind _asbp_quadditch_game_mode (Utilities|Casting|CastToBP_Quadditch_Game_Mode (Game|GetGameMode)))
    (Default|IncrementScore _asbp_quadditch_game_mode (Utilities|Select :Index _owning_team :NewEnumerator0 "NewEnumerator1" :NewEnumerator1 "NewEnumerator0"))
    (Actor|DestroyActor _array_element)
    (CallFunction|HoopEffects)
    (CallFunction|RestoreBall)))

(fn ConstructionScript
  (Rendering|Material|SetVectorParameterValueonMaterials (Variables|Default|GetStaticMesh) "Color" (Utilities|Select :Index (Variables|Default|Getowning_team) :NewEnumerator0 "1.000000,0.000000,0.000000" :NewEnumerator1 "0.000000,0.000000,1.000000")))